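; Projectile Blueprint that is sized and given its launch speed in the Construction Script.
; The script stretches the actor's X and Z scale and adds the instigator's speed, as a velocity magnitude, to the ProjectileMovement initial speed.
; The Hit event is empty; the dust emitter and actor destruction logic is disconnected and never runs.
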(event Collision|EventHit
  (params (MyComp :type Primitive%20Component%20Object%20Reference) (Other :type Actor%20Object%20Reference) (OtherComp :type Primitive%20Component%20Object%20Reference) (bSelfMoved :type Boolean) (HitLocation :type Vector) (HitNormal :type Vector :default "0, 0, 0") (NormalImpulse :type Vector :default "0, 0, 0") (Hit :type Hit%20Result%20Structure%20%28by%20ref%29)))

(fn ConstructionScript
  (bind _projectilemovement (Variables|Default|GetProjectileMovement))
  (Transformation|SetActorScale3D "1.400000,1.000000,1.400000")
  (Variables|/Script/Engine.ProjectileMovementComponent|SetInitialSpeed _projectilemovement (+ (Variables|/Script/Engine.ProjectileMovementComponent|GetInitialSpeed _projectilemovement) (Math|Vector|VectorLength (Transformation|GetVelocity (Game|GetInstigator))))))