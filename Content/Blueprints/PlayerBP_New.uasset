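; Player character for a 2D Paper2D side-scroller, with movement, crawl and look-up states, wall jumps and air jumps.
; Tick drives sprite flip and tilt, aim and an AltFire scanner that picks the closest scannable in a forward cone.
; Timelines add bobbing and landing squash, and capsule overlaps track camera boundary volumes.
; The flipbook state machine update, double-jump limit, dust and projectile spawning are disconnected.
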(event OnFinishedPlaying(Sprite)
  ;[1 256 256] Anim Control
  ;;[348.3 1 1] One-shots handler
  (switch string (stale _currentanimationstring)
    (:Default
      _)
    (:Jump
      (Variables|AnimationStates|SetJumping false))
    (:LookUp
      (Variables|AnimationStates|SetLookUpStatic true)))
  (Components|Timeline|SetLooping (Variables|Default|GetSprite) true))

(event OnComponentEndOverlap(CapsuleComponent)
  (params (OverlappedComponent :type Primitive%20Component%20Object%20Reference) (OtherActor :type Actor%20Object%20Reference) (OtherComp :type Primitive%20Component%20Object%20Reference) (OtherBodyIndex :type Integer))
  ;[1 1 1] Track Camera Boundaries
  (bind _ascamera_blocking_volume (Utilities|Casting|CastToCameraBlockingVolume OtherActor))
  (Utilities|Array|RemoveItem (Variables|Default|GetCurrentCameraBoundaries) _ascamera_blocking_volume))

(event OnComponentBeginOverlap(CapsuleComponent)
  (params (OverlappedComponent :type Primitive%20Component%20Object%20Reference) (OtherActor :type Actor%20Object%20Reference) (OtherComp :type Primitive%20Component%20Object%20Reference) (OtherBodyIndex :type Integer) (bFromSweep :type Boolean) (SweepResult :type Hit%20Result%20Structure%20%28by%20ref%29))
  ;[1 1 1] Track Camera Boundaries
  (bind _ascamera_blocking_volume (Utilities|Casting|CastToCameraBlockingVolume OtherActor))
  (Utilities|Array|AddUnique (Variables|Default|GetCurrentCameraBoundaries) _ascamera_blocking_volume))

(event Custom|WallJump
  (bind _returnvalue (Transformation|GetActorLocation))
  (bind _walljumpxvelocity (Variables|Default|GetWallJumpXVelocity))
  ;[1 1 1] WallJump Logic
  (bind (_outhit _returnvalue_2) (Collision|LineTraceByChannel (Math|Vector|MakeVector (- (- (.x _returnvalue) (Components|Capsule|GetScaledCapsuleRadius (Variables|Collision|GetCapsuleComponent))) (Variables|Default|GetWallJumpRaycastLength)) (.y _returnvalue) (.z _returnvalue)) (Math|Vector|MakeVector (+ (.x _returnvalue) (Variables|Default|GetWallJumpRaycastLength) (Components|Capsule|GetScaledCapsuleRadius (Variables|Collision|GetCapsuleComponent))) (.y _returnvalue) (.z _returnvalue)) "TraceTypeQuery1" false 0 "None"))
  (if _returnvalue_2
    (Character|LaunchCharacter (Math|Vector|MakeVector (* (Math|Float|Sign(Float) (- (.x (Transformation|GetActorLocation)) (.x (.Location (Collision|BreakHitResult _outhit))))) (Math|Float|SelectFloat _walljumpxvelocity (* _walljumpxvelocity 0.5) (== (Math|Float|Absolute(Float) (+ (Math|Float|Sign(Float) (- (.x (Transformation|GetActorLocation)) (.x (.Location (Collision|BreakHitResult _outhit))))) (Input|AxisValues|GetMoveRight))) 2.0))) 0.0 (Variables|/Script/Engine.CharacterMovementComponent|GetJumpZVelocity (Variables|Character|GetCharacterMovement))) false true)
    (CallFunction|JumpFX)
    (Variables|AnimationStates|SetJumping true)
    (else
      (CallFunction|DoubleJump))))

(event Custom|UpdateAnim
  ;[1 256 256] Anim Control
)

(event Custom|DoubleJump
  ;[1 1 1] DoubleJump mid-air if no collision
  (Character|LaunchCharacter "0, 0,500.000000" false true)
  (CallFunction|JumpFX)
  (Variables|Default|SetCanDoubleJump false)
  (Variables|AnimationStates|SetJumping true))

(event Custom|RotateOnSpeed
  (bind _sprite (Variables|Default|GetSprite))
  (bind _returnvalue (Transformation|GetWorldRotation _sprite))
  ;[1 1 1] Flip X Axis on Input
  (if (> (Math|Float|Absolute(Float) (.x (Transformation|GetVelocity))) 0.0)
    (Transformation|SetRelativeRotation _sprite (Math|Rotator|MakeRotator 0.0 -15.0 (.yaw _returnvalue)) false false)
    (else
      (Transformation|SetRelativeRotation _sprite (Math|Rotator|MakeRotator 0.0 0.0 (.yaw _returnvalue)) false false))))

(event Custom|JumpFX
  ;[1 1 1] Jump n Land FX
)

(event Custom|ScanComplete
  (bind _closestscannable (Variables|Scanner|GetClosestScannable))
  ;[1 0 0.9975] SCANNER
  ;;[1 1 1] Initiate scan and accumulate scannables withing range
  (Variables|Scanner|SetClosestScannableDistance 1e+03)
  (Utilities|FlowControl|DoOnce false) ; enters at Reset
)

(event Custom|GetClosestScannable
  (bind _scannablesinrange (Variables|Scanner|GetScannablesInRange))
  ;[1 0 0.9975] SCANNER
  ;;[1 1 1] Get the closest scannable and apply state to it
  (if (!= (Utilities|Array|Length _scannablesinrange) 0)
    (for _array_element _scannablesinrange
      (Math|Float|CompareFloat (Math|Vector|VectorLength (- (Transformation|GetActorLocation _array_element) (Transformation|GetActorLocation))) (Variables|Scanner|GetClosestScannableDistance)
        (:==
          _)
        (:<
          _))
      (Utilities|IsValid (Variables|Scanner|GetClosestScannable) ; Avoid error
        (:Is%20Valid
          _)
        (:Is%20Not%20Valid
          _))
      (Variables|Scanner|SetClosestScannable _array_element)
      (Variables|Scanner|SetClosestScannableDistance (Math|Vector|VectorLength (- (Transformation|GetActorLocation _array_element) (Transformation|GetActorLocation)))))
    (Default|ScanMeEvent (Variables|Scanner|GetClosestScannable))
    (CallFunction|ScanComplete)
    (else
      (CallFunction|ScanComplete))))

(event Custom|DoScan
  (params (DeltaTime :type Float%20%28single-precision%29))
  (bind _closestscannable (Variables|Scanner|GetClosestScannable))
  ;[1 0 0.9975] SCANNER
  ;;[1 1 1] Initiate scan and accumulate scannables withing range
  (if (Variables|Scanner|GetisScanning)
    (Utilities|FlowControl|DoOnce false
      (:Completed
        (Utilities|FlowControl|Sequence
          (:then_0
            (Utilities|Array|Clear (Variables|Scanner|GetScannablesInRange)) ; Clear list of scannables in range
            (for _array_element (Variables|Scanner|GetScannableObjects)
              (Variables|Scanner|SetCurrentScannable _array_element)
              (if (and (>= (Math|Vector|DotProduct (* (Transformation|GetActorForwardVector) (Math|Float|SelectFloat 1.0 -1.0 (Variables|AnimationStates|GetfacingRight))) (Math|Vector|Normalize (- (Transformation|GetActorLocation (Variables|Scanner|GetCurrentScannable)) (Transformation|GetWorldLocation (Variables|Default|GetProjectileLocator))))) 0.5) (<= (Math|Vector|VectorLength (- (Transformation|GetActorLocation (Variables|Scanner|GetCurrentScannable)) (Transformation|GetWorldLocation (Variables|Default|GetProjectileLocator)))) 1.5e+02)) ; In range check
                (Utilities|Array|AddUnique (Variables|Scanner|GetScannablesInRange) (Variables|Scanner|GetCurrentScannable))
                (else
                  (Default|ResetEvent (Variables|Scanner|GetCurrentScannable)))))
            (CallFunction|GetClosestScannable))
          (:then_1
            (goto _label Reset)))))
    (else
      ;;[1 1 1] Reset closest scannable when stop scanning
      (Utilities|FlowControl|DoOnce true :!label _label
        (:Completed
          (Utilities|IsValid _closestscannable
            (:Is%20Valid
              (Default|ResetEvent _closestscannable))))))))

(event Custom|LandFX
  ;[1 1 1] Jump n Land FX
  (Utilities|FlowControl|Sequence
    (:then_0
      (bind _jump (Timeline|Timeline_0 PlayFromStart)
        (:Update
          (Transformation|SetActorScale3D (Math|Vector|Lerp(Vector) "1.000000,1.000000,1.000000" "2.000000,1.000000,0.500000" (* _jump 0.6))))))))

(event Custom|PrintDebug
  (params (DeltaTime :type Float%20%28single-precision%29))
  (Development|PrintString "Hello" true true "(R=0.000000,G=0.660000,B=1.000000,A=1.000000)" DeltaTime))

(event Custom|CheckFlip
  (bind _sprite (Variables|Default|GetSprite))
  ;[1 1 1] Flip X Axis on Input
  (Math|Float|CompareFloat (Input|AxisValues|GetMoveRight) 0.0
    (:>
      (Transformation|SetRelativeRotation _sprite "0, 0, 0" false false)
      (Variables|AnimationStates|SetfacingRight true))
    (:<
      (Transformation|SetRelativeRotation _sprite "0,180.000000, 0" false false)
      (Variables|AnimationStates|SetfacingRight false))))

(event Custom|UpdateFireDirection
  ;[1 1 1] Aim
  (if (Variables|AnimationStates|GetLookUpStatic)
    (Transformation|SetRelativeRotation (Variables|Default|GetProjectileLocator) "90.000000, 0, 0" false false)
    (else
      (Transformation|SetRelativeRotation (Variables|Default|GetProjectileLocator) "0.000000, 0, 0" false false))))

(event EventBeginPlay
  ;[1 1 1] Bobbing Animation
  (Components|Timeline|SetPlayRate (Variables|Default|GetBobbingTimeline) (Variables|BobbingAnimation|GetBobbing_PlayRate))
  (bind _location (Timeline|BobbingTimeline Play)
    (:Update
      (Transformation|SetRelativeLocation (Variables|Default|GetSprite) (* _location (Variables|BobbingAnimation|GetBobbingAmount)) false false))))

(event EventOnLanded
  (params (Hit :type Hit%20Result%20Structure%20%28by%20ref%29))
  ;[1 1 1] Jumping
  (Variables|Default|SetCanDoubleJump true)
  (CallFunction|LandFX))

(event EventTick
  (params (DeltaSeconds :type Float%20%28single-precision%29))
  ;[1 1 256] Tick
  (CallFunction|DoScan DeltaSeconds)
  (CallFunction|PrintDebug DeltaSeconds)
  (CallFunction|UpdateAnim)
  (CallFunction|CheckFlip)
  (CallFunction|UpdateFireDirection)
  (CallFunction|RotateonSpeed))

(event Input|ActionEvents|InputActionJump
  (params (Key :type Key%20Structure :default "AnyKey"))
  ;[1 1 1] Jumping
  (:Pressed
    (Character|Jump)
    (if (AI|Components|NavMovement|IsFalling (Variables|Character|GetCharacterMovement))
      (CallFunction|WallJump)
      (else
        (CallFunction|JumpFX)
        (Variables|AnimationStates|SetJumping true))))
  (:Released
    (Character|StopJumping)))

(event Input|ActionEvents|InputActionFire
  (params (Key :type Key%20Structure :default "AnyKey")))

(event Input|ActionEvents|InputActionAltFire
  (params (Key :type Key%20Structure :default "AnyKey"))
  (:Pressed
    (Variables|Scanner|SetisScanning true))
  (:Released
    (Variables|Scanner|SetisScanning false)))

(event Input|AxisEvents|InputAxisMoveRight
  (params (AxisValue :type Float%20%28single-precision%29))
  ;[1 256 1] Move sideways
  (Pawn|Input|AddMovementInput "1.000000, 0, 0" AxisValue false))

(event Input|AxisEvents|InputAxisCrawl
  (params (AxisValue :type Float%20%28single-precision%29))
  ;[1 256 1] Check Crawl
  (Math|Float|CompareFloat AxisValue 0.0
    (:>
      (Variables|AnimationStates|SetCrawling true))
    (:==
      (Variables|AnimationStates|SetCrawling false))))

(event Input|AxisEvents|InputAxisUp
  (params (AxisValue :type Float%20%28single-precision%29))
  ;[1 256 1] Check LookUp
  (Math|Float|CompareFloat AxisValue 0.0
    (:>
      (Variables|AnimationStates|SetLookUp true))
    (:==
      (Variables|AnimationStates|SetLookUp false)
      (Variables|AnimationStates|SetLookUpStatic false))))

(fn ConstructionScript
  (Variables|Default|SetPlayerCamera 0)
  (Variables|/Script/Engine.CharacterMovementComponent|SetJumpZVelocity (Variables|Character|GetCharacterMovement) 4e+02)
  (Variables|Default|SetJumpMaxHoldTime 0.3))

(fn AnimationStateMachine
  (params (Walking :type Boolean) (Jumping :type Boolean) (Falling :type Boolean) (LookingUp :type Boolean) (LookingUpStatic :type Boolean) (Crawling :type Boolean) (Sprite :type Paper%20Flipbook%20Component%20Object%20Reference))
  ;[1 1 1] Jumping
  (if Jumping
    (Components|Timeline|SetLooping Sprite false)
    (LocalVariables|SetAnimState "NewEnumerator2")
    (else
      ;[1 1 1] Falling
      (if Falling
        (LocalVariables|SetAnimState "NewEnumerator6")
        (else
          ;[1 1 1] Crawl Walk
          (if (and Crawling Walking)
            (LocalVariables|SetAnimState "NewEnumerator10")
            (else
              ;[1 1 1] Crawl Idle
              (if Crawling
                (LocalVariables|SetAnimState "NewEnumerator9")
                (else
                  ;[1 1 1] Walking
                  (if Walking
                    (LocalVariables|SetAnimState "NewEnumerator1")
                    (else
                      ;[1 1 1] LookUpStatic
                      (if LookingUpStatic
                        (LocalVariables|SetAnimState "NewEnumerator8")
                        (else
                          ;[1 1 1] Lookup
                          (if LookingUp
                            (Components|Timeline|SetLooping Sprite false)
                            (LocalVariables|SetAnimState "NewEnumerator7")
                            (else
                              (LocalVariables|SetAnimState "NewEnumerator0")))))))))))))))
  (return (Utilities|Select :Index (LocalVariables|GetAnimState) :NewEnumerator0 "/Game/Art/Flipbooks/HerIdle.HerIdle" :NewEnumerator1 "/Game/Art/Flipbooks/HeroWalk.HeroWalk" :NewEnumerator2 "/Game/Art/Flipbooks/HeroJump.HeroJump" :NewEnumerator6 "/Game/Art/Flipbooks/Falling.Falling" :NewEnumerator7 "/Game/Art/Flipbooks/LookUp.LookUp" :NewEnumerator8 "/Game/Art/Flipbooks/LookUpStatic.LookUpStatic" :NewEnumerator9 "/Game/Art/Flipbooks/Crouching_Idle.Crouching_Idle" :NewEnumerator10 "/Game/Art/Flipbooks/Crouching_Walk.Crouching_Walk") (Utilities|String|EnumtoString (LocalVariables|GetAnimState))))