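; Scannable Blueprint with a Paper2D sprite that changes color as it is scanned and reveals its scan text when complete.
; Each ScanMe_Event call increments ScanValue, clamps and normalizes it over a 0–100 range, and lerps the sprite from BaseColor to ScanColor.
; At full progress it prints ScanText, using Tick's DeltaSeconds as the display duration.
; Reset_Event zeroes progress and sets the sprite to white rather than BaseColor.
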(event Custom|ScanMe_Event
  (bind _result (Math|Float|IncrementFloat (Variables|Default|GetScanValue))
    (:%20%20
      (Sprite|SetSpriteColor (Variables|Default|GetPaperSprite) (Math|Color|Lerp(LinearColor) (Variables|Default|GetBaseColor) (Variables|Default|GetScanColor) (Math|Float|NormalizetoRange (Math|Float|Clamp(Float) _result 0.0 1e+02) 0.0 1e+02)))
      (Math|Float|CompareFloat (Math|Float|NormalizetoRange (Math|Float|Clamp(Float) _result 0.0 1e+02) 0.0 1e+02) 1.0
        (:==
          (Development|PrintString (Variables|Default|GetScanText) true true "(R=0.000000,G=0.660000,B=1.000000,A=1.000000)" (stale EventTick DeltaSeconds)))))))

(event Custom|Reset_Event
  (Sprite|SetSpriteColor (Variables|Default|GetPaperSprite) "(R=1.000000,G=1.000000,B=1.000000,A=1.000000)")
  (Variables|Default|SetScanValue 0.0))

(event EventTick
  (params (DeltaSeconds :type Float%20%28single-precision%29)))

(fn ConstructionScript)